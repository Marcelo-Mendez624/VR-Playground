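; BP_Saber is a saber actor that slices procedural meshes its blade passes through and awards score to the BP_SPawn player pawn.
; Blade begin overlap caches the procedural mesh and adds score.
; End overlap slices it along PointComponent's location and up vector with a capped cut, then launches both halves with physics impulses.
; If the exiting component is the cached mesh, its actor is hidden and removed after a short delay.
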(event OnComponentBeginOverlap(Blade)
  (params (OverlappedComponent :type Primitive%20Component%20Object%20Reference) (OtherActor :type Actor%20Object%20Reference) (OtherComp :type Primitive%20Component%20Object%20Reference) (OtherBodyIndex :type Integer) (bFromSweep :type Boolean) (SweepResult :type Hit%20Result%20Structure%20%28by%20ref%29))
  ;[1 1 1] Slice
  (Variables|Default|SetProceduralMeshRef 0)
  (bind _asprocedural_mesh_component (Utilities|Casting|CastToProceduralMeshComponent OtherComp))
  (Variables|Default|SetProceduralMeshRef _asprocedural_mesh_component)
  (bind _asbp_spawn (Utilities|Casting|CastToBP_SPawn (Game|Player|GetPlayerPawn 0)))
  (Variables|/Game/_VRPORTFOLIO/Blueprints/BP_SPawn.BP_SPawn_C|SetScore _asbp_spawn (+ (Variables|/Game/_VRPORTFOLIO/Blueprints/BP_SPawn.BP_SPawn_C|GetScore _asbp_spawn) 10)))

(event OnComponentEndOverlap(Blade)
  (params (OverlappedComponent :type Primitive%20Component%20Object%20Reference) (OtherActor :type Actor%20Object%20Reference) (OtherComp :type Primitive%20Component%20Object%20Reference) (OtherBodyIndex :type Integer))
  (bind _pointcomponent (Variables|Default|GetPointComponent))
  (bind _proceduralmeshref (Variables|Default|GetProceduralMeshRef))
  (bind _proceduralmeshref_2 (Variables|Default|GetProceduralMeshRef))
  ;[1 1 1] Slice
  (Utilities|IsValid (Variables|Default|GetProceduralMeshRef)
    (:Is%20Valid
      (bind _outotherhalfprocmesh (Class|KismetProceduralMeshLibrary|SliceProceduralMesh (stale OnComponentBeginOverlap(Blade) _asprocedural_mesh_component) (Transformation|GetWorldLocation _pointcomponent) (Math|Vector|GetUpVector _pointcomponent) true "CreateNewSectionForCap" "/Game/_VRPORTFOLIO/Materials/M_Saber_Inst.M_Saber_Inst"))
      (Physics|SetSimulatePhysics _proceduralmeshref true)
      (Physics|AddImpulse _proceduralmeshref "-150.000000,-100.000000,100.000000" "None" true)
      (Physics|SetSimulatePhysics _outotherhalfprocmesh true)
      (Physics|AddImpulse _outotherhalfprocmesh "200.000000,200.000000,50.000000" "None" true)
      (Collision|SetCollisionEnabled _proceduralmeshref_2 "PhysicsOnly")
      (if (== _proceduralmeshref_2 OtherComp)
        (Utilities|FlowControl|Delay 0.4)
        (Rendering|SetActorHiddenInGame OtherActor true)
        (Components|DestroyComponent _outotherhalfprocmesh)
        (Actor|SetLifeSpan OtherActor 0.1)))))

(event EventBeginPlay)

(fn ConstructionScript)